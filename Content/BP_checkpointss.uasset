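; Checkpoint actor for a flight race in GM_FlightTest, collected in index order through an overlap trigger.
; On overlap, a checkpoint matching the game mode's current index advances the index and count, then destroys itself.
; The first checkpoint starts the race, and reaching the total count finishes it.
; The game mode is told to update checkpoint visibility, and SetIndicatorVisible toggles this checkpoint's indicator arrow.
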(event `self.Triggerchecked.OnComponentBeginOverlap`
  (params (OverlappedComponent :type "PrimitiveComponent Object Reference") (OtherActor :type "Actor Object Reference") (OtherComp :type "PrimitiveComponent Object Reference") (OtherBodyIndex :type Integer) (bFromSweep :type Boolean) (SweepResult :type "HitResult Structure (by ref)"))
  (bind _gmref (`self.GMRef`))
  (bind _gmref_2 (`self.GMRef`))
  ; CollectCheckpoint
  (bind _asgm_flight_test (cast `/Game/GM_FlightTest` (`GameplayStatics.GetGameMode`)))
  (`KismetSystemLibrary.PrintString` "Hello")
  (bind _output_get (set `self.GMRef` _asgm_flight_test))
  (bind _currentcheckpointindex (`/Game/GM_FlightTest.CurrentCheckpointIndex` _output_get))
  (if (== (`self.CheckpointIndex`) _currentcheckpointindex)
    (bind _output_get_2 (set `/Game/GM_FlightTest.NextCheckpointIndex` (+ _currentcheckpointindex 1) _output_get))
    (set `self.ISfirstcheckpoint` (== _currentcheckpointindex 1))
    (set `/Game/GM_FlightTest.CurrentCheckpointIndex` _output_get_2 _output_get)
    (set `/Game/GM_FlightTest.CheckpointsCollected` (+ (`/Game/GM_FlightTest.CheckpointsCollected` _gmref_2) 1) _gmref_2)
    (if (`self.ISfirstcheckpoint`)
      (`/Game/GM_FlightTest.StartRace` (`self.GMRef`))
      (`KismetSystemLibrary.PrintString` "RACE STARTED"))
    (if (== (`/Game/GM_FlightTest.CheckpointsCollected` _gmref) (`/Game/GM_FlightTest.TotalCheckpoints` _gmref))
      (`KismetSystemLibrary.PrintString` "HOW TF")
      (`/Game/GM_FlightTest.FinishRace` (`self.GMRef`)))
    (`/Game/GM_FlightTest.UpdateCheckpointVisibility` (`self.GMRef`))
    (`self.K2_DestroyActor`)))

(fn `SetIndicatorVisible`
  (params (bVisible :type Boolean))
  (`KismetSystemLibrary.PrintString` (`KismetStringLibrary.Conv_BoolToString` bVisible))
  (`SceneComponent.SetVisibility` (`self.Indicator Arrow`) bVisible true))

(fn `UserConstructionScript`)