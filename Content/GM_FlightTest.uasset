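; Game mode for a flight checkpoint race that tracks race state, times the run and briefly shows the pawn's finish screen.
; BeginPlay shows only checkpoint 1's indicator after a short delay.
; Update events unhide a window of upcoming checkpoints and highlight the current one, using an AllCheckpoints array that is not filled here.
; FindNextCheckpoint searches all checkpoint actors for NextCheckpointIndex, ignoring its PlayerLocation input.
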(event `self.ReceiveBeginPlay`
  (`KismetSystemLibrary.Delay` 0.2)
  (bind _outactors (`GameplayStatics.GetAllActorsOfClass` "/Game/BP_checkpoint.BP_checkpoint_C"))
  (for _array_element _outactors
    (if (== (`/Game/BP_checkpoint.CheckpointIndex` _array_element) 1)
      (`/Game/BP_checkpoint.SetIndicatorVisible` _array_element true)
      (else
        (`/Game/BP_checkpoint.SetIndicatorVisible` _array_element false)))))

(event `StartRace`
  (set `self.RaceStartTime` (`KismetSystemLibrary.GetGameTimeInSeconds`))
  (set `self.RaceActive` true)
  (`KismetSystemLibrary.PrintString` "Race Started"))

(event `FinishRace`
  (bind _output_get (set `self.FinalTime` (- (`KismetSystemLibrary.GetGameTimeInSeconds`) (`self.RaceStartTime`))))
  (set `self.RaceActive` false)
  (`KismetSystemLibrary.PrintString` (`KismetStringLibrary.Conv_DoubleToString` _output_get))
  (bind _returnvalue (`GameplayStatics.GetActorOfClass` "/Game/Blueprints/BP_MyPawn.BP_MyPawn_C"))
  (`/Game/Blueprints/BP_MyPawn.FinishScreen` _returnvalue true)
  (`KismetSystemLibrary.Delay` 6.0)
  (`/Game/Blueprints/BP_MyPawn.FinishScreen` _returnvalue false))

(event `UpdateCheckpointVisibility`
  (for _array_element (`self.AllCheckpoints`)
    (`/Engine/EditorBlueprintResources/StandardMacros.IsValid` _array_element
      (:`Is Valid`
        (bind _checkpointindex (`/Game/BP_checkpoint.CheckpointIndex` _array_element))
        (if (and (< _checkpointindex (+ (`self.CurrentCheckpointIndex`) (`self.VisibleAhead`))) (>= _checkpointindex (`self.CurrentCheckpointIndex`)))
          (`self.SetActorHiddenInGame` _array_element false)
          (else
            (`self.SetActorHiddenInGame` _array_element true)))))))

(event `UpdateIndicatorVisibility`
  (for _array_element (`self.AllCheckpoints`)
    (`/Engine/EditorBlueprintResources/StandardMacros.IsValid` _array_element
      (:`Is Valid`
        (if (== (`/Game/BP_checkpoint.CheckpointIndex` _array_element) (`self.CurrentCheckpointIndex`))
          (`/Game/BP_checkpoint.SetIndicatorVisible` _array_element true)
          (else
            (`/Game/BP_checkpoint.SetIndicatorVisible` _array_element false)))))))

(fn `FindNextCheckpoint`
  (params (PlayerLocation :type "Vector Structure"))
  (returns (NextCheckpoint :type "/Game/BP_checkpoint Object Reference"))
  (bind _outactors (`GameplayStatics.GetAllActorsOfClass` "/Game/BP_checkpoint.BP_checkpoint_C"))
  (for _array_element _outactors
    (`/Engine/EditorBlueprintResources/StandardMacros.IsValid` _array_element
      (:`Is Valid`
        (if (== (`/Game/BP_checkpoint.CheckpointIndex` _array_element) (`self.NextCheckpointIndex`))
          (return _array_element)))
      (:`Is Not Valid`
        (`KismetSystemLibrary.PrintString` "ISNOTVALID")))))

(fn `UserConstructionScript`)