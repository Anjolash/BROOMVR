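; BP_CheckpointTrack is a spline-based track actor that populates a course with checkpoints for the GM_FlightTest game mode.
; On BeginPlay it spawns checkpoint actors at even spacing along TrackSpline, inset by a start/finish buffer and oriented to the spline.
; Each gets a 1-based index and is registered with the game mode, which then receives the total count and refreshes checkpoint visibility.
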(event `self.ReceiveBeginPlay`
  (bind _gmref (`self.GMRef`))
  ; Track Logic
  (set `self.SplineLength` (`SplineComponent.GetSplineLength` (`self.TrackSpline`)))
  (bind _asgm_flight_test (cast `/Game/GM_FlightTest` (`GameplayStatics.GetGameMode`)))
  (set `self.GMRef` _asgm_flight_test)
  (bind _output_get (set `self.TotalCount` (`KismetMathLibrary.FFloor` (/ (- (`self.SplineLength`) (* (`self.StartFinishBuffer`) 2.0)) (`self.SpacingDistance`)))))
  (for _index (range _output_get)
    (set `self.CurrentDistance` (+ (* _index (`self.SpacingDistance`)) (`self.StartFinishBuffer`)))
    (bind _returnvalue (`|SpawnActorFromClass` (`self.CheckpointClass`) (`KismetMathLibrary.MakeTransform` (`SplineComponent.GetLocationAtDistanceAlongSpline` (`self.TrackSpline`) (`self.CurrentDistance`) "World") (`SplineComponent.GetRotationAtDistanceAlongSpline` (`self.TrackSpline`) (`self.CurrentDistance`) "World")) "Undefined" "MultiplyWithRoot" null 0 null))
    (bind _output_get_2 (set `self.SpawnedCheckpoint` _returnvalue))
    (set `/Game/BP_checkpoint.CheckpointIndex` (+ _index 1) _output_get_2)
    (`KismetArrayLibrary.Array_Add` (`/Game/GM_FlightTest.AllCheckpoints` (`self.GMRef`)) _returnvalue))
  (set `/Game/GM_FlightTest.TotalCheckpoints` (`self.TotalCount`) _gmref)
  (`/Game/GM_FlightTest.UpdateCheckpointVisibility` _gmref))

(fn `UserConstructionScript`)