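; BP_Ballon is a balloon actor with a purely cosmetic idle floating motion.
; Each tick it sets the relative location and rotation of MeshRoot from sine waves of game time.
; A slow sine bobs it vertically, while two layered sines at different frequencies sway its yaw back and forth.
; It has no other active logic.
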(event `self.ReceiveTick`
  (params (DeltaSeconds :type "Float (single-precision)"))
  (bind _returnvalue (`KismetSystemLibrary.GetGameTimeInSeconds`))
  (`SceneComponent.K2_SetRelativeLocationAndRotation` (`self.Mesh Root`) (`KismetMathLibrary.MakeVector` 0.0 0.0 (* (`KismetMathLibrary.Sin` (* _returnvalue 0.5)) 10.0)) (`KismetMathLibrary.MakeRotator` 0.0 0.0 (+ (* (`KismetMathLibrary.Sin` (* _returnvalue 0.2)) 10.0) (* (`KismetMathLibrary.Sin` (* _returnvalue 1.0)) 1.0))) false false))

(fn `UserConstructionScript`)