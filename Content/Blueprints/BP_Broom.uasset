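; BP_Broom is a VR broom actor with separate left-hand and right-hand grab points.
; Each of its two grab components responds only to its matching hand, swapping that hand mesh's material and setting a HoldingL or HoldingR flag on grab and drop.
; It also toggles that hand's message on the VR pawn, reached through the motion controller's owner to avoid a hard pawn reference.
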(event `self.BP_GrabComponent1.OnGrabbed`
  (bind _bp_grabcomponent1 (`self.BP_GrabComponent1`))
  (if (`|EnumEquality` (`/Game/XRFramework/Blueprints/BP_GrabComponent.GetHeldByHand` (`self.BP_GrabComponent1`)) "Left")
    (`PrimitiveComponent.SetMaterial` (`self.Hand_L`) 0 "/Engine/EngineDebugMaterials/LevelColorationUnlitMaterial.LevelColorationUnlitMaterial")
    (set `self.Holding_L` true)
    (message `/Game/XRFramework/Blueprints/BPI_PawnAnim.HideUnhideHand` (`ActorComponent.GetOwner` (`/Game/XRFramework/Blueprints/BP_GrabComponent.MotionControllerRef` _bp_grabcomponent1)) true (`|EnumEquality` (`/Game/XRFramework/Blueprints/BP_GrabComponent.GetHeldByHand` _bp_grabcomponent1) "Right"))))

(event `self.BP_GrabComponent1.OnDropped`
  (bind _bp_grabcomponent1 (`self.BP_GrabComponent1`))
  (if (`|EnumEquality` (`/Game/XRFramework/Blueprints/BP_GrabComponent.GetHeldByHand` (`self.BP_GrabComponent1`)) "Left")
    (`PrimitiveComponent.SetMaterial` (`self.Hand_L`) 0 "/Engine/BasicShapes/BasicShapeMaterial.BasicShapeMaterial")
    (set `self.Holding_L` false)
    (message `/Game/XRFramework/Blueprints/BPI_PawnAnim.HideUnhideHand` (`ActorComponent.GetOwner` (`/Game/XRFramework/Blueprints/BP_GrabComponent.MotionControllerRef` _bp_grabcomponent1)) false (`|EnumEquality` (`/Game/XRFramework/Blueprints/BP_GrabComponent.GetHeldByHand` _bp_grabcomponent1) "Right"))))

(event `self.BP_GrabComponent2.OnGrabbed`
  (bind _bp_grabcomponent2 (`self.BP_GrabComponent2`))
  (if (`|EnumEquality` (`/Game/XRFramework/Blueprints/BP_GrabComponent.GetHeldByHand` (`self.BP_GrabComponent2`)) "Right")
    (`PrimitiveComponent.SetMaterial` (`self.Hand_R`) 0 "/Engine/EngineDebugMaterials/LevelColorationUnlitMaterial.LevelColorationUnlitMaterial")
    (set `self.Holding_R` true)
    (message `/Game/XRFramework/Blueprints/BPI_PawnAnim.HideUnhideHand` (`ActorComponent.GetOwner` (`/Game/XRFramework/Blueprints/BP_GrabComponent.MotionControllerRef` _bp_grabcomponent2)) true (`|EnumEquality` (`/Game/XRFramework/Blueprints/BP_GrabComponent.GetHeldByHand` _bp_grabcomponent2) "Right"))))

(event `self.BP_GrabComponent2.OnDropped`
  (bind _bp_grabcomponent2 (`self.BP_GrabComponent2`))
  (if (`|EnumEquality` (`/Game/XRFramework/Blueprints/BP_GrabComponent.GetHeldByHand` (`self.BP_GrabComponent2`)) "Right")
    (`PrimitiveComponent.SetMaterial` (`self.Hand_R`) 0 "/Engine/BasicShapes/BasicShapeMaterial.BasicShapeMaterial")
    (set `self.Holding_R` false)
    (message `/Game/XRFramework/Blueprints/BPI_PawnAnim.HideUnhideHand` (`ActorComponent.GetOwner` (`/Game/XRFramework/Blueprints/BP_GrabComponent.MotionControllerRef` _bp_grabcomponent2)) false (`|EnumEquality` (`/Game/XRFramework/Blueprints/BP_GrabComponent.GetHeldByHand` _bp_grabcomponent2) "Right"))))

(fn `UserConstructionScript`)