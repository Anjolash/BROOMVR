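; Game mode for a flight test race that tracks race state and timing and controls which checkpoints are visible.
; StartRace and FinishRace toggle the active flag, store game-time timestamps and print debug messages; FinalTime holds raw game time, without subtracting the start time.
; UpdateCheckpointVisibility shows only a sliding window of VisibleAhead checkpoints from the current index, hiding all others.
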(event `StartRace`
  (set `self.RaceStartTime` (`KismetSystemLibrary.GetGameTimeInSeconds`))
  (set `self.RaceActive` true)
  (`KismetSystemLibrary.PrintString` "Race Started"))

(event `FinishRace`
  (bind _output_get (set `self.FinalTime` (`KismetSystemLibrary.GetGameTimeInSeconds`)))
  (set `self.RaceActive` false)
  (`KismetSystemLibrary.PrintString` (`KismetStringLibrary.Conv_DoubleToString` _output_get)))

(event `UpdateCheckpointVisibility`
  (for _array_element (`self.AllCheckpoints`)
    (bind _checkpointindex (`/Game/BP_checkpoint.CheckpointIndex` _array_element))
    (if (and (< _checkpointindex (+ (`self.CurrentCheckpointIndex`) (`self.VisibleAhead`))) (>= _checkpointindex (`self.CurrentCheckpointIndex`)))
      (`self.SetActorHiddenInGame` _array_element false)
      (else
        (`self.SetActorHiddenInGame` _array_element true)))))

(fn `UserConstructionScript`)